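; Bullet projectile actor that destroys itself when it slows down or hits an enemy vehicle.
; A short delay after BeginPlay arms a speed check on Tick, which destroys the bullet once its Sphere component moves below a velocity threshold.
; Overlapping a VehicleBlueprinEnemy actor destroys it immediately, with no damage applied here.
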(event `self.ReceiveBeginPlay`
  (`KismetSystemLibrary.Delay` 0.2)
  (set `self.timer` true))

(event `self.ReceiveTick`
  (params (DeltaSeconds :type "Float (single-precision)"))
  (if (`self.timer`)
    (if (< (`KismetMathLibrary.VSize` (`SceneComponent.GetComponentVelocity` (`self.Sphere`))) 200.0)
      (`self.K2_DestroyActor` :!label _label))))

(event `self.ReceiveActorBeginOverlap`
  (params (OtherActor :type "Actor Object Reference"))
  (if (== (`GameplayStatics.GetObjectClass` OtherActor) "/Game/VehicleAdvBP/Blueprints/VehicleBlueprinEnemy.VehicleBlueprinEnemy_C")
    (goto _label)))

(fn `UserConstructionScript`)